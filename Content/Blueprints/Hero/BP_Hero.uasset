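; Player hero character that handles look, move and jump through Enhanced Input and the Gameplay Ability System.
; BeginPlay adds the default mapping context and grants GA_Jump, which the jump input activates by class.
; Look drives controller yaw and pitch, while movement follows control rotation with pitch ignored.
; Landing sends a GameplayEvent.OnLanded event to itself, so abilities can react to touchdown.
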(event Input|EnhancedActionEvents|EnhancedInputActionIA_Look
  (params (ActionValue :type Vector%202D%20Structure) (ElapsedSeconds :type Float%20%28double-precision%29) (TriggeredSeconds :type Float%20%28double-precision%29) (InputAction :type Input%20Action%20Object%20Reference :default "/Game/Input/Actions/IA_Look.IA_Look"))
  (Input|CameraInputs (.x ActionValue) (.y ActionValue)))

(event Input|EnhancedActionEvents|EnhancedInputActionIA_Move
  (params (ActionValue :type Vector%202D%20Structure) (ElapsedSeconds :type Float%20%28double-precision%29) (TriggeredSeconds :type Float%20%28double-precision%29) (InputAction :type Input%20Action%20Object%20Reference :default "/Game/Input/Actions/IA_Move.IA_Move"))
  (Input|MovementInputs (.x ActionValue) (.y ActionValue)))

(event Input|EnhancedActionEvents|EnhancedInputActionIA_Jump
  (params (ActionValue :type Boolean) (ElapsedSeconds :type Float%20%28double-precision%29) (TriggeredSeconds :type Float%20%28double-precision%29) (InputAction :type Input%20Action%20Object%20Reference :default "/Game/Input/Actions/IA_Jump.IA_Jump"))
  (:Started
    (Abilities|TryActivateAbilitybyClass (Variables|Default|GetAbilitySystemComponent) "/Game/Blueprints/GameplayAbilities/GA_Jump.GA_Jump_C" true)))

(event EventBeginPlay
  (Utilities|FlowControl|Sequence
    (:then_0
      (Input|InitializeEnhancedInput))
    (:then_1
      (GameplayAbilities|GiveAbility (Variables|Default|GetAbilitySystemComponent) "/Game/Blueprints/GameplayAbilities/GA_Jump.GA_Jump_C" 0 -1))))

(event EventOnLanded
  (params (Hit :type Hit%20Result%20Structure%20%28by%20ref%29))
  (Ability|SendGameplayEventtoActor self "(TagName=\"GameplayEvent.OnLanded\")"))

(fn ConstructionScript
  (|CallParentFunction))

(fn InitializeEnhancedInput
  (bind _asplayer_controller (Utilities|Casting|CastToPlayerController (Pawn|GetController)))
  (Utilities|IsValid (PlayerController|LocalPlayerSubsystems|GetEnhancedInputLocalPlayerSubsystem _asplayer_controller)
    (:Is%20Valid
      (Input|AddMappingContext (PlayerController|LocalPlayerSubsystems|GetEnhancedInputLocalPlayerSubsystem _asplayer_controller) "/Game/Input/IMC_Default.IMC_Default" 0 "(bIgnoreAllPressedKeysUntilRelease=True,bForceImmediately=False,bNotifyUserSettings=False)"))))

(fn CameraInputs
  (params (Yaw :type Float%20%28single-precision%29) (Pitch :type Float%20%28single-precision%29))
  (Pawn|Input|AddControllerYawInput Yaw)
  (Pawn|Input|AddControllerPitchInput Pitch))

(fn MovementInputs
  (params (LeftRight :type Float%20%28double-precision%29) (ForwardBackward :type Float%20%28double-precision%29))
  (bind _returnvalue (Pawn|GetControlRotation :!class /Script/Engine.Pawn))
  (Pawn|Input|AddMovementInput (Math|Vector|GetRightVector (Math|Rotator|MakeRotator (.roll _returnvalue) 0.0 (.yaw _returnvalue))) LeftRight false)
  (Pawn|Input|AddMovementInput (Math|Vector|GetForwardVector (Math|Rotator|MakeRotator 0.0 0.0 (.yaw (Pawn|GetControlRotation :!class /Script/Engine.Pawn)))) ForwardBackward false))