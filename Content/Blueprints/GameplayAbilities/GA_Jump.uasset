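; GA_Jump is a Gameplay Ability that makes the avatar Character jump.
; On activation it commits, casts the avatar to Character and calls Jump, cancelling itself if either the commit or the cast fails.
; It stays active until a GameplayEvent.OnLanded event reaches the character, then ends.
; On end it prints a string showing whether it was cancelled or ended normally.
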(event Ability|EventActivateAbility
  (bind _returnvalue (Ability|CommitAbility))
  (if _returnvalue
    (bind _ascharacter (Utilities|Casting|CastToCharacter (Ability|GetAvatarActorfromActorInfo))
      (:then
        (bind _output_get (Variables|Default|SetAvatarCharacter _ascharacter))
        (Character|Jump _output_get)
        (Ability|Async|WaitGameplayEventToActor _output_get "(TagName=\"GameplayEvent.OnLanded\")"
          (:EventReceived
            (Ability|EndAbility))))
      (:CastFailed
        (Ability|CancelAbility :!label _label)))
    (else
      (goto _label))))

(event Ability|EventOnEndAbility
  (params (bWasCancelled :type Boolean))
  (Development|PrintString (select bWasCancelled "Cancel Ability" "End Ability")))